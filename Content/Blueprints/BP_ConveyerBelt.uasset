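; Conveyor belt actor that charges the level's battery according to how far its player, found by PlayerIndex, is along the belt.
; Each Tick, the player's X distance from the start, divided by the belt length cached at BeginPlay, accumulates into SCORE and feeds ChargeBattery.
; Charging requires being past the start; the end-point check is disconnected.
; Player and battery references resolve lazily in Tick, and construction counter-scales the Arrow.
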(event EventBeginPlay
  (bind _conveyorstart (Variables|Default|GetConveyorStart))
  (bind _conveyorend (Variables|Default|GetConveyorEnd))
  (bind _returnvalue (Transformation|GetWorldLocation _conveyorstart))
  (bind _returnvalue_2 (Transformation|GetWorldLocation _conveyorend))
  ;[1 1 1] Caching Conveyor, start and end points of conveyor, needed for battery Z-axis response.
  (Variables|Conveyor|SetLocationStart _returnvalue)
  (Variables|Conveyor|SetLocationEnd _returnvalue_2)
  (Variables|Conveyor|SetDistance (Math|Vector|Distance(Vector) _returnvalue _returnvalue_2)))

(event EventTick
  (params (DeltaSeconds :type Float%20%28single-precision%29))
  ;[1 1 1] Battery behaviour
  (Utilities|IsValid (Variables|References|GetPlayerCharacterRef) ; Constantly checks if the player instance is valid.
    (:Is%20Valid
      (Utilities|IsValid (Variables|References|GetBatteryRef)
        (:Is%20Valid
          ;;[1 1 1] Gets the battery class in the level, check if it's valid, then sends the SCORE of the player (SCORE + 1) + M.
          (bind _output_get (Variables|Conveyor|SetMultiplier (/ (Math|Vector|Distance(Vector) (Math|Vector|MakeVector (.x (Transformation|GetActorLocation (Variables|References|GetPlayerCharacterRef))) 0.0 0.0) (Math|Vector|MakeVector (.x (Variables|Conveyor|GetLocationStart)) 0.0 0.0)) (Variables|Conveyor|GetDistance)))) ; Sets the multiplier (between 0 and 1) for the value of SCORE being sent to the battery for each player.
          (Variables|Conveyor|SetSCORE (+ _output_get (Variables|Conveyor|GetSCORE)))
          ;;[1 1 1] Checks if the player character has exceeded either the start or end points.
          (if (not (<= (.x (Transformation|GetWorldLocation (Variables|/Script/Engine.Actor|GetRootComponent (Variables|References|GetPlayerCharacterRef)))) (.x (Transformation|GetWorldLocation (Variables|Default|GetConveyorStart)))))
            (Default|ChargeBattery (Variables|References|GetBatteryRef) _output_get)
            (Development|PrintString (Utilities|String|ToString(Float) _output_get) true true "(R=0.007223,G=1.000000,B=0.000000,A=1.000000)" 0.0)))
        (:Is%20Not%20Valid
          (bind _outactors (Actor|GetAllActorsOfClass "/Game/Blueprints/BP_Battery.BP_Battery_C"))
          (Utilities|IsValid (Utilities|Array|Get(acopy) _outactors)
            (:Is%20Valid
              (Variables|References|SetBatteryRef (Utilities|Array|Get(acopy) _outactors)))))))
    (:Is%20Not%20Valid
      (bind _asbp_cbplayer (Utilities|Casting|CastToBP_CBPlayer (Game|Player|GetPlayerPawn (Variables|References|GetPlayer%20Index))))
      (Variables|References|SetPlayerCharacterRef _asbp_cbplayer))))

(fn ConstructionScript
  (Transformation|SetRelativeScale3D (Variables|Default|GetArrow) (/ "1.000000,1.000000,1.000000" (Transformation|GetActorScale3D))))