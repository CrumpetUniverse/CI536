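; Player controller for the overworld that turns each player's gamepad D-pad and bottom face button presses into directional and confirm actions.
; BeginPlay caches the CI536 overworld Game Mode and this controller's player ID, then passes that ID with every input call to the Game Mode.
; BeginPlay and each successful action refresh the overworld player pawn's Credits text from that player's Game Instance data.
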(event EventBeginPlay
  ;[1 1 1] Cache the Game Mode and Player Controller ID
  (bind _asci536overworld_game_mode_base (Utilities|Casting|CastToCI536OverworldGameModeBase (Game|GetGameMode)))
  (Variables|Default|SetOverworldGameMode _asci536overworld_game_mode_base)
  (Variables|Default|SetPlayerControllerID (Class|GameplayStatics|GetPlayerControllerID self))
  (bind _asbp_overworld_player (Utilities|Casting|CastToBP_OverworldPlayer (Game|Player|GetPlayerPawn (Variables|Default|GetPlayerControllerID))))
  (bind _asci536game_instance (Utilities|Casting|CastToCI536GameInstance (Game|GetGameInstance)))
  (Rendering|Components|TextRender|SetText (Variables|/Game/Blueprints/BP_OverworldPlayer.BP_OverworldPlayer_C|GetCredits _asbp_overworld_player) (Utilities|Text|ToText(Integer) (.credits (Utilities|Array|Get(acopy) (Variables|/Script/CI536.CI536GameInstance|GetPlayerInformation _asci536game_instance) (Variables|Default|GetPlayerControllerID))))))

(event Input|GamepadEvents|GamepadFaceButtonBottom
  (params (Key :type Key%20Structure))
  (bind _playercontrollerid (Variables|Default|GetPlayerControllerID))
  ;[1 1 1] Confirm
  (:Pressed
    (bind _overworldgamemode (Variables|Default|GetOverworldGameMode)
      (:then
        (bind _returnvalue (Class|CI536OverworldGameModeBase|Confirm _overworldgamemode (Variables|Default|GetPlayerControllerID)))
        (if _returnvalue
          (bind _asbp_overworld_player (Utilities|Casting|CastToBP_OverworldPlayer (Game|Player|GetPlayerPawn _playercontrollerid)))
          (bind _asci536game_instance (Utilities|Casting|CastToCI536GameInstance (Game|GetGameInstance)))
          (Rendering|Components|TextRender|SetText (Variables|/Game/Blueprints/BP_OverworldPlayer.BP_OverworldPlayer_C|GetCredits _asbp_overworld_player) (Utilities|Text|ToText(Integer) (.credits (Utilities|Array|Get(acopy) (Variables|/Script/CI536.CI536GameInstance|GetPlayerInformation _asci536game_instance) _playercontrollerid))))))
      (:else))))

(event Input|GamepadEvents|GamepadDPadUp
  (params (Key :type Key%20Structure))
  (bind _playercontrollerid (Variables|Default|GetPlayerControllerID))
  ;[1 1 1] Nortrh
  (:Pressed
    (bind _overworldgamemode (Variables|Default|GetOverworldGameMode)
      (:then
        (bind _returnvalue (Class|CI536OverworldGameModeBase|North _overworldgamemode (Variables|Default|GetPlayerControllerID)))
        (if _returnvalue
          (bind _asbp_overworld_player (Utilities|Casting|CastToBP_OverworldPlayer (Game|Player|GetPlayerPawn _playercontrollerid)))
          (bind _asci536game_instance (Utilities|Casting|CastToCI536GameInstance (Game|GetGameInstance)))
          (Rendering|Components|TextRender|SetText (Variables|/Game/Blueprints/BP_OverworldPlayer.BP_OverworldPlayer_C|GetCredits _asbp_overworld_player) (Utilities|Text|ToText(Integer) (.credits (Utilities|Array|Get(acopy) (Variables|/Script/CI536.CI536GameInstance|GetPlayerInformation _asci536game_instance) _playercontrollerid))))))
      (:else))))

(event Input|GamepadEvents|GamepadDPadRight
  (params (Key :type Key%20Structure))
  (bind _playercontrollerid (Variables|Default|GetPlayerControllerID))
  ;[1 1 1] East
  (:Pressed
    (bind _overworldgamemode (Variables|Default|GetOverworldGameMode)
      (:then
        (bind _returnvalue (Class|CI536OverworldGameModeBase|East _overworldgamemode (Variables|Default|GetPlayerControllerID)))
        (if _returnvalue
          (bind _asbp_overworld_player (Utilities|Casting|CastToBP_OverworldPlayer (Game|Player|GetPlayerPawn _playercontrollerid)))
          (bind _asci536game_instance (Utilities|Casting|CastToCI536GameInstance (Game|GetGameInstance)))
          (Rendering|Components|TextRender|SetText (Variables|/Game/Blueprints/BP_OverworldPlayer.BP_OverworldPlayer_C|GetCredits _asbp_overworld_player) (Utilities|Text|ToText(Integer) (.credits (Utilities|Array|Get(acopy) (Variables|/Script/CI536.CI536GameInstance|GetPlayerInformation _asci536game_instance) _playercontrollerid))))))
      (:else))))

(event Input|GamepadEvents|GamepadDPadDown
  (params (Key :type Key%20Structure))
  (bind _playercontrollerid (Variables|Default|GetPlayerControllerID))
  ;[1 1 1] South
  (:Pressed
    (bind _overworldgamemode (Variables|Default|GetOverworldGameMode)
      (:then
        (bind _returnvalue (Class|CI536OverworldGameModeBase|South _overworldgamemode (Variables|Default|GetPlayerControllerID)))
        (if _returnvalue
          (bind _asbp_overworld_player (Utilities|Casting|CastToBP_OverworldPlayer (Game|Player|GetPlayerPawn _playercontrollerid)))
          (bind _asci536game_instance (Utilities|Casting|CastToCI536GameInstance (Game|GetGameInstance)))
          (Rendering|Components|TextRender|SetText (Variables|/Game/Blueprints/BP_OverworldPlayer.BP_OverworldPlayer_C|GetCredits _asbp_overworld_player) (Utilities|Text|ToText(Integer) (.credits (Utilities|Array|Get(acopy) (Variables|/Script/CI536.CI536GameInstance|GetPlayerInformation _asci536game_instance) _playercontrollerid))))))
      (:else))))

(event Input|GamepadEvents|GamepadDPadLeft
  (params (Key :type Key%20Structure))
  (bind _playercontrollerid (Variables|Default|GetPlayerControllerID))
  ;[1 1 1] West
  (:Pressed
    (bind _overworldgamemode (Variables|Default|GetOverworldGameMode)
      (:then
        (bind _returnvalue (Class|CI536OverworldGameModeBase|West _overworldgamemode (Variables|Default|GetPlayerControllerID)))
        (if _returnvalue
          (bind _asbp_overworld_player (Utilities|Casting|CastToBP_OverworldPlayer (Game|Player|GetPlayerPawn _playercontrollerid)))
          (bind _asci536game_instance (Utilities|Casting|CastToCI536GameInstance (Game|GetGameInstance)))
          (Rendering|Components|TextRender|SetText (Variables|/Game/Blueprints/BP_OverworldPlayer.BP_OverworldPlayer_C|GetCredits _asbp_overworld_player) (Utilities|Text|ToText(Integer) (.credits (Utilities|Array|Get(acopy) (Variables|/Script/CI536.CI536GameInstance|GetPlayerInformation _asci536game_instance) _playercontrollerid))))))
      (:else))))

(fn ConstructionScript)