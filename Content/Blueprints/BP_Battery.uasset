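; Battery actor that charges up, rising from its starting location and switching on a light when full.
; ChargeBattery adds a charge increment scaled by delta time, a factor and the inverse of the GameMode's player controller count, clamped to 0–1.
; It then lerps the root's height by that charge up to an offset.
; Tick uses a resetting DoOnce to reveal the light once at full charge.
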(event EventBeginPlay
  ;[1 1 1] Begin Play: Cahce the GameMode and the battery's location.
  (bind _asci536game_mode_base (Utilities|Casting|CastToCI536GameModeBase (Game|GetGameMode)))
  (Variables|Default|SetGameMode _asci536game_mode_base)
  (Variables|Default|SetLocation (Transformation|GetActorLocation)))

(event EventTick
  (params (DeltaSeconds :type Float%20%28single-precision%29))
  ;[1 1 1] Tick: If the battery is fully charged, turn the light on.
  (Utilities|FlowControl|DoOnce false :!label _label
    (:Completed
      (if (>= (Variables|Default|GetCharge) 1.0)
        (Rendering|SetVisibility (Variables|Default|GetLight) true false)
        (else
          (goto _label Reset))))))

(fn ConstructionScript)

(fn ChargeBattery
  (params (Charge :type Float%20%28single-precision%29))
  (bind _output_get (Variables|Default|SetCharge (Math|Float|Clamp(Float) (+ (Variables|Default|GetCharge) (* (* (/ Charge (Math|Conversions|ToFloat(Integer) (Variables|/Script/CI536.CI536GameModeBase|GetPlayerControllerCount (Variables|Default|GetGameMode)))) (Utilities|Time|GetWorldDeltaSeconds)) (Variables|Default|GetFactor))))))
  (Transformation|SetWorldLocation (Variables|Default|GetDefaultSceneRoot) (Math|Vector|Lerp(Vector) (Variables|Default|GetLocation) (+ (Variables|Default|GetLocation) (Math|Vector|MakeVector 0.0 0.0 (Variables|Default|GetOffset))) _output_get) false false))