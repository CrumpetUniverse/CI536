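; Player character for the conveyor minigame, where mashing the ButtonMash input pushes against a growing backward drift.
; Each press adds Factor to Force, which Tick decays toward zero and applies as a world X nudge with a constant negative bias.
; Tick also moves the actor opposite the capsule's forward vector at a speed that grows every frame.
; Movement skips sweeps, and only decay and drift use DeltaSeconds.
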(event EventTick
  (params (DeltaSeconds :type Float%20%28single-precision%29))
  (bind _capsulecomponent (Variables|Collision|GetCapsuleComponent))
  ;[1 1 1] Updates world location based on input
  (bind _output_get (Variables|Default|SetForce (Math|Float|Lerp (Variables|Default|GetForce) 0.0 DeltaSeconds)))
  (Transformation|SetWorldLocation _capsulecomponent (+ (Transformation|GetWorldLocation _capsulecomponent) (Math|Vector|MakeVector (* (+ _output_get -1.0) 0.5) 0.0 0.0)) false false)
  (Variables|Default|SetCurrentSpeed (+ (Variables|Default|GetCurrentSpeed) (Variables|Default|GetAcceleration)))
  (Transformation|AddActorLocalOffset (* (* (Math|Rotator|GetRotationXVector (Transformation|GetWorldRotation (Variables|Collision|GetCapsuleComponent))) (* DeltaSeconds (Variables|Default|GetCurrentSpeed))) -1.0) false false))

(event Input|ActionEvents|InputActionButtonMash
  (params (Key :type Key%20Structure :default "None"))
  ;[1 1 1] Player Movement for the conveyor game - mashing of the input event (SPACE / A / LR Triggers)
  (:Pressed
    (Variables|Default|SetForce (+ (Variables|Default|GetForce) (Variables|Default|GetFactor)))))

(fn ConstructionScript)