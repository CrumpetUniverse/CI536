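; Game mode for local multiplayer that creates players and switches them between a game pawn and a spawn pawn.
; BeginPlay caches all PlayerStarts and creates local players until the count exceeds three.
; Spawn and despawn events destroy a controller's valid pawn, possess the replacement and set the view to a shared Camera.
; Both take transforms from RandomSpawn, whose random PlayerStart lookup appears unconnected.
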(event Custom|SpawnPlayer
  (params (PlayerController :type Player%20Controller%20Object%20Reference))
  (bind _returnvalue (Pawn|GetControlledPawn PlayerController))
  ;[1 1 1] Spawn Player
  (Utilities|IsValid _returnvalue
    (:Is%20Valid
      (Actor|DestroyActor _returnvalue)
      (bind _returnvalue_2 (Game|SpawnActorfromClass "/Game/Characters/ConveyorGame/Blueprints/ConveyorGame_Pawntest.ConveyorGame_Pawntest_C" (Utilities|RandomSpawn) "Undefined" 0 0))
      (Pawn|Possess PlayerController _returnvalue_2)
      (Game|Player|SetViewTargetwithBlend PlayerController (Variables|Default|GetCamera) 0.0 "VTBlend_Linear" 0.0 false))))

(event Custom|DespawnPlayer
  (params (PlayerController :type Player%20Controller%20Object%20Reference))
  (bind _returnvalue (Pawn|GetControlledPawn PlayerController))
  ;[1 1 1] Despawn Player
  (Utilities|IsValid _returnvalue
    (:Is%20Valid
      (Actor|DestroyActor _returnvalue)
      (bind _returnvalue_2 (Game|SpawnActorfromClass "/Game/Base/Blueprints/SpawnPawn.SpawnPawn_C" (Utilities|RandomSpawn) "Undefined" 0 0))
      (Pawn|Possess PlayerController _returnvalue_2)
      (Game|Player|SetViewTargetwithBlend PlayerController (Variables|Default|GetCamera) 0.0 "VTBlend_Linear" 0.0 false))))

(event EventBeginPlay
  ;[1 1 1] Spawns
  (bind _outactors (Actor|GetAllActorsOfClass "/Script/Engine.PlayerStart"))
  (Variables|Default|SetSpawns _outactors)
  (while (<= (Variables|Default|GetNumberOfPlayers) 3)
    (Variables|Default|SetNumberOfPlayers (+ (Variables|Default|GetNumberOfPlayers) 1))
    (Class|GameplayStatics|CreatePlayer -1)))

(fn ConstructionScript)