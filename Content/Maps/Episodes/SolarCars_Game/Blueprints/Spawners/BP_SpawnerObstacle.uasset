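; Spawner Blueprint for the SolarCars game that drops obstacles at its own location at random intervals.
; On BeginPlay it caches the level manager, then loops a random delay between min and max bounds and a placement, repeating while the manager reports play is active.
; Spawning defers to the parent class, and spawned obstacles that hit the bounds are destroyed.
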(event Custom|LineUpNextObstacleSpawn
  (Utilities|FlowControl|Delay (Math|Random|RandomFloatinRange (Variables|Default|GetMinDelay) (Variables|Default|GetMaxDelay)))
  (CallFunction|PlaceObstacle)
  (if (Variables|/Game/Maps/Episodes/SolarCars_Game/Blueprints/Game/BP_SolarCars_LevelManager.BP_SolarCars_LevelManager_C|GetbIsPlaying (Variables|Default|GetLevelManagerRef))
    (CallFunction|LineUpNextObstacleSpawn)))

(event EventBeginPlay
  (bind (_levelmanager _levelmanagerfound) (CallFunction|GetLevelManager))
  (|CallParentFunction)
  (if _levelmanagerfound
    (Variables|Default|SetLevelManagerRef _levelmanager)
    (CallFunction|LineUpNextObstacleSpawn)))

(fn ConstructionScript
  (|CallParentFunction))

(fn PlaceObstacle
  (bind _returnvalue (CallFunction|SpawnActor))
  (Transformation|SetActorLocation _returnvalue (Transformation|GetActorLocation) false false))

(fn SpawnActor
  (bind _returnvalue (|CallParentFunction))
  (return _returnvalue))

(fn SpawnedActorHitBounds
  (params (OutOfBoundsActor :type Actor%20Object%20Reference))
  (|CallParentFunction 0)
  (Actor|DestroyActor OutOfBoundsActor))