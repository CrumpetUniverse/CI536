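; Level manager for the SolarCars game, holding level speed and play state along with a bounds box meant to recycle items that go out of bounds.
; The construction script sizes and positions LevelBounds from the out-of-bound scale and location variables.
; Actors that begin overlapping the box return a parent, which is notified through SpawnedActorHitBounds.
; GameOver zeroes the level speed and clears the playing flag.
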(event OnComponentBeginOverlap(LevelBounds)
  (params (OverlappedComponent :type Primitive%20Component%20Object%20Reference) (OtherActor :type Actor%20Object%20Reference) (OtherComp :type Primitive%20Component%20Object%20Reference) (OtherBodyIndex :type Integer) (bFromSweep :type Boolean) (SweepResult :type Hit%20Result%20Structure%20%28by%20ref%29))
  (bind _parent (Class|BPInterfaceSpawner|ReturnParent(Message) OtherActor))
  (Utilities|IsValid _parent
    (:Is%20Valid
      (Default|SpawnedActorHitBounds _parent OtherActor))))

(fn ConstructionScript
  (bind _levelbounds (Variables|Default|GetLevelBounds))
  ;[1 1 1] OutOfBound should basically remove items past this bounds (recycler)
  (Components|Box|SetBoxExtent _levelbounds (Variables|Default|GetOutOfBoundBoxScale) true)
  (Transformation|SetWorldLocation _levelbounds (Variables|Default|GetOutOfBoundBoxLocation) false false))

(fn GameOver
  (Variables|Default|SetLevelSpeed 0.0)
  (Variables|Default|SetbIsPlaying false))