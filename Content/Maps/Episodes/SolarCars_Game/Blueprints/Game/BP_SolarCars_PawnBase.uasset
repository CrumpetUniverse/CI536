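; Base player pawn for the SolarCars lane-dodging game that slides sideways between lanes on Left and Right input.
; On BeginPlay it finds the Level Manager, takes its lane width and starts in the middle lane.
; While the manager reports play is active, input runs timelines that lerp Y one lane over, blocked at outer lanes and during a move.
; HitObstacle toggles the mesh's visibility.
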(event EventBeginPlay
  (bind (_levelmanager _levelmanagerfound) (CallFunction|GetLevelManager))
  ;[1 1 1] We could colapse this to the function, but for better clarity I kept it like this
  (if _levelmanagerfound
    (Variables|Default|SetLevelManagerRef _levelmanager)
    (Variables|Default|SetCurrent%20Lane (+ (/ (Variables|/Game/Maps/Episodes/SolarCars_Game/Blueprints/Game/BP_SolarCars_LevelManager.BP_SolarCars_LevelManager_C|GetNumberOfLanes (Variables|Default|GetLevelManagerRef)) 2) 1))
    (Variables|Default|SetLane%20Width (Variables|/Game/Maps/Episodes/SolarCars_Game/Blueprints/Game/BP_SolarCars_LevelManager.BP_SolarCars_LevelManager_C|GetLaneWidth (Variables|Default|GetLevelManagerRef)))
    (else
      (Development|PrintString "No Level Manager Found"))))

(event Input|ActionEvents|InputActionLeft
  (params (Key :type Key%20Structure))
  (bind _returnvalue (Transformation|GetActorLocation))
  (:Pressed
    ;[1 1 1] Obstacle Hit check
    (if (Variables|/Game/Maps/Episodes/SolarCars_Game/Blueprints/Game/BP_SolarCars_LevelManager.BP_SolarCars_LevelManager_C|GetbIsPlaying (Variables|Default|GetLevelManagerRef))
      ;[1 1 1] If we pressed left and have been already in the left most lane
      (if (not (<= (Variables|Default|GetCurrent%20Lane) 1))
        ;[1 1 1] Comment
        (if (not (Variables|Default|GetbMoving))
          (Variables|Default|SetbMoving true)
          (Variables|Default|SetTargetPosition (- (.y (Transformation|GetActorLocation)) (Variables|Default|GetLane%20Width)))
          (bind _move (Timeline|MoveLeft PlayFromStart)
            (:Update
              (Transformation|SetActorLocation (Math|Vector|MakeVector (.x _returnvalue) (Math|Float|Lerp (.y _returnvalue) (Variables|Default|GetTargetPosition) _move) (.z _returnvalue)) false false))
            (:Finished
              (Variables|Default|SetbMoving false)
              (Math|Integer|DecrementInt (Variables|Default|GetCurrent%20Lane)))))))))

(event Input|ActionEvents|InputActionRight
  (params (Key :type Key%20Structure))
  (bind _returnvalue (Transformation|GetActorLocation))
  (:Pressed
    ;[1 1 1] Obstacle Hit Check
    (if (Variables|/Game/Maps/Episodes/SolarCars_Game/Blueprints/Game/BP_SolarCars_LevelManager.BP_SolarCars_LevelManager_C|GetbIsPlaying (Variables|Default|GetLevelManagerRef))
      ;[1 1 1] Check if we pressed Right in the Right most lane
      (if (not (== (Variables|Default|GetCurrent%20Lane) (Variables|/Game/Maps/Episodes/SolarCars_Game/Blueprints/Game/BP_SolarCars_LevelManager.BP_SolarCars_LevelManager_C|GetNumberOfLanes (Variables|Default|GetLevelManagerRef))))
        (if (not (Variables|Default|GetbMoving))
          (Variables|Default|SetbMoving true)
          (Variables|Default|SetTargetPosition (+ (.y (Transformation|GetActorLocation)) (Variables|Default|GetLane%20Width)))
          (bind _move (Timeline|MoveRight PlayFromStart)
            (:Update
              (Transformation|SetActorLocation (Math|Vector|MakeVector (.x _returnvalue) (Math|Float|Lerp (.y _returnvalue) (Variables|Default|GetTargetPosition) _move) (.z _returnvalue)) false false))
            (:Finished
              (Variables|Default|SetbMoving false)
              (Math|Integer|IncrementInt (Variables|Default|GetCurrent%20Lane)))))))))

(fn ConstructionScript)

(fn HitObstacle
  (Rendering|ToggleVisibility (Variables|Default|GetStaticMesh) false))