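; BP_FloorBaseObsolete is a floor base actor, marked obsolete by name, that scrolls at the level's speed in the SolarCars game.
; On BeginPlay it caches the Level Manager reference if valid.
; Each Tick it scales its forward vector by the manager's LevelSpeed and delta time, then applies that world-space vector as a local offset without sweep.
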(event EventBeginPlay
  (bind _output (Utilities|GetLevelManager)
    (:Is%20Valid
      (Variables|Default|SetLevelManagerRef _output))))

(event EventTick
  (params (DeltaSeconds :type Float%20%28single-precision%29))
  (Variables|Default|SetDeltaSeconds DeltaSeconds)
  (bind _output_get (Variables|Default|SetMovement (* (* (Transformation|GetActorForwardVector) (Variables|/Game/Maps/Episodes/SolarCars_Game/Blueprints/Game/BP_SolarCars_LevelManager.BP_SolarCars_LevelManager_C|GetLevelSpeed (Variables|Default|GetLevelManagerRef))) (Variables|Default|GetDeltaSeconds))))
  (Transformation|AddActorLocalOffset _output_get false false))

(fn ConstructionScript)