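; Battery actor for the conveyor minigame that charges from player input and lights up when full.
; ChargeBattery scales incoming charge by player count, frame time and a factor, clamps the total to 0–1, and lerps the root vertically from its starting position.
; Tick uses a resettable DoOnce to show the battery light at full charge.
; AddScore only prints the score it receives.
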(event EventBeginPlay
  ;[1 1 1] Cache the number of players
  (bind _asci536game_mode_base (Utilities|Casting|CastToCI536GameModeBase (Game|GetGameMode)))
  (Variables|Default|SetGameMode _asci536game_mode_base)
  (Variables|Default|SetOrigin (Transformation|GetWorldLocation (Variables|Default|GetDefaultSceneRoot))))

(event Collision|EventActorBeginOverlap
  (params (OtherActor :type Actor%20Object%20Reference)))

(event EventTick
  (params (DeltaSeconds :type Float%20%28single-precision%29))
  (Utilities|FlowControl|DoOnce false :!label _label
    (:Completed
      (if (>= (Variables|Default|GetCharge) 1.0)
        (Rendering|SetVisibility (Variables|Default|GetBatteryLight) true false)
        (else
          (goto _label Reset))))))

(fn ConstructionScript)

(fn AddScore
  (params (SCORE :type Float%20%28single-precision%29))
  ;[1 1 1] Battery takes the score from each player. Divides it by the number of players in the session.
  (Development|PrintString (Utilities|String|ToString(Float) SCORE)))

(fn ChargeBattery
  (params (Charge :type Float%20%28single-precision%29))
  (bind _gamemode (Variables|Default|GetGameMode))
  (bind _playercontrollercount (Variables|/Script/CI536.CI536GameModeBase|GetPlayerControllerCount _gamemode))
  (bind _returnvalue (Math|Conversions|ToFloat(Integer) _playercontrollercount))
  (bind _returnvalue_2 (/ Charge _returnvalue))
  (bind _output_get (Variables|Default|SetCharge (Math|Float|Clamp(Float) (+ (Variables|Default|GetCharge) (* (* _returnvalue_2 (Utilities|Time|GetWorldDeltaSeconds)) (Variables|Default|GetFactor))))))
  (Transformation|SetWorldLocation (Variables|Default|GetDefaultSceneRoot) (Math|Vector|Lerp(Vector) (Variables|Default|GetOrigin) (+ (Variables|Default|GetOrigin) (Math|Vector|MakeVector 0.0 0.0 (Variables|Default|GetOffset))) _output_get) false false)
  (Development|PrintString (Utilities|String|ToString(Float) _returnvalue_2) true true "(R=1.000000,G=0.982638,B=0.000000,A=1.000000)" 0.0))