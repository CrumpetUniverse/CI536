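; BP_Button is a button that unifies mouse hover and keyboard focus into one visual selection state.
; Initialise starts a looping timer that polls Update every tenth of a second instead of binding to hover or focus events.
; Update gives a hovered button keyboard focus and the mouse style, otherwise applying the selected or not-selected style depending on whether it holds keyboard focus.
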(fn Initialise
  (Utilities|Time|SetTimerbyFunctionName 0 "Update" 0.1 true))

(fn Update
  (if (Widget|IsHovered)
    (Widget|SetKeyboardFocus)
    (Class|Button|SetStyle (Variables|Default|GetStyleMouse))
    (else
      (Class|Button|SetStyle (select (Class|Widget|HasKeyboardFocus) (Variables|Default|GetStyleSelected) (Variables|Default|GetStyleNotSelected))))))